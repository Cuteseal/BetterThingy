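; Zombie enemy AI that chases the player and deals damage when close.
; Pawn sensing triggers AI movement toward a seen player unless the player is inside the attack radius overlap volume.
; A timeline started at BeginPlay serves as the attack loop, using delays to pace health loss and briefly set the player's TakingDamage flag.
; Tick destroys the zombie once its health runs out.
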(event OnComponentBeginOverlap(AttackRadius)
  (params (OverlappedComponent :type Primitive%20Component%20Object%20Reference) (OtherActor :type Actor%20Object%20Reference) (OtherComp :type Primitive%20Component%20Object%20Reference) (OtherBodyIndex :type Integer) (bFromSweep :type Boolean) (SweepResult :type Hit%20Result%20Structure%20%28by%20ref%29))
  ;[1 1 1] Checking if Player is in attack radius
  (Utilities|Casting|CastToPlayer OtherActor)
  (Variables|Default|Setis%20in%20attack%20radius true))

(event OnComponentEndOverlap(AttackRadius)
  (params (OverlappedComponent :type Primitive%20Component%20Object%20Reference) (OtherActor :type Actor%20Object%20Reference) (OtherComp :type Primitive%20Component%20Object%20Reference) (OtherBodyIndex :type Integer))
  ;[1 1 1] Checking if Player is in attack radius
  (Utilities|Casting|CastToPlayer OtherActor)
  (Variables|Default|Setis%20in%20attack%20radius false))

(event OnSeePawn(PawnSensing)
  (params (Pawn :type Pawn%20Object%20Reference))
  (if (not (Variables|Default|Getis%20in%20attack%20radius))
    (bind _asplayer (Utilities|Casting|CastToPlayer Pawn))
    (AI|AIMoveTo self "0, 0, 0" _asplayer 5.0 false)))

(event EventBeginPlay
  ;[1 1 1] Beginplay
  ;[1 1 1] Attacking player
  (Timeline|Timeline_0 Play
    (:Update
      (if (Variables|Default|Getis%20in%20attack%20radius)
        (bind _asplayer (Utilities|Casting|CastToPlayer (Game|GetPlayerCharacter 0)))
        (if (not (<= (Variables|/Game/Blueprints/Player/Player.Player_C|GetHealth _asplayer) 0.0))
          (Utilities|FlowControl|Delay 0.7)
          (bind _asplayer_2 (Utilities|Casting|CastToPlayer (Game|GetPlayerCharacter 0)))
          (Utilities|FlowControl|Sequence
            (:then_0
              (Variables|/Game/Blueprints/Player/Player.Player_C|SetHealth _asplayer_2 (- (Variables|/Game/Blueprints/Player/Player.Player_C|GetHealth _asplayer_2) 0.25)))
            (:then_1
              (Variables|/Game/Blueprints/Player/Player.Player_C|SetTaking%20Damage _asplayer_2 true)
              (Utilities|FlowControl|Delay 0.2)
              (Variables|/Game/Blueprints/Player/Player.Player_C|SetTaking%20Damage _asplayer_2 false))))))))

(event EventTick
  (params (DeltaSeconds :type Float%20%28single-precision%29))
  ;[1 1 1] Tick
  ;[1 1 1] Damage
  (if (<= (Variables|Default|GetHealth) 0.0)
    (Actor|DestroyActor)))

(fn ConstructionScript)